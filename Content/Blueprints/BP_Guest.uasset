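; BP_Guest is a guest actor that can be picked up and placed on a seat.
; Interact flags it as grabbed and moves it to a fixed world location near the origin, without releasing any seat it holds.
; TrySitAt moves it to a valid, free seat's Box location, links guest and seat, marks the seat occupied and clears the grab.
; Invalid or occupied seats only print a debug message.
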(event `/Game/Blueprints/BPI_Interactable.Interact`
  (set `self.IsGrabbed` true)
  (`self.K2_SetActorLocation` (0.0 0.0 50.0)))

(fn `TrySitAt`
  (params (TargetSeat :type "/Game/Blueprints/BP_Seat Object Reference"))
  (if (`KismetSystemLibrary.IsValid` TargetSeat)
    (if (`/Game/Blueprints/BP_Seat.IsOccupied` TargetSeat)
      (`KismetSystemLibrary.PrintString` "IsOccupied")
      (else
        (`self.K2_SetActorLocation` self (`SceneComponent.K2_GetComponentLocation` (`/Game/Blueprints/BP_Seat.Box` TargetSeat)) false false)
        (set `self.CurrentSeat` TargetSeat)
        (set `/Game/Blueprints/BP_Seat.IsOccupied` true TargetSeat)
        (set `/Game/Blueprints/BP_Seat.Occupany` self TargetSeat)
        (set `self.IsGrabbed` false)))
    (else
      (`KismetSystemLibrary.PrintString` "SeatIsInvalid" true true (struct :`R` 1.0 :`G` 0.040103 :`A` 1.0)))))

(fn `UserConstructionScript`)